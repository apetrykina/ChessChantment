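; AR player pawn that places a game board on a detected real-world surface when the screen is touched.
; A touch first runs WorldHitTest, a deprojected object trace that blocks placement if it hits existing world objects.
; Otherwise an AR tracked-object trace, excluding feature points and ground plane, supplies the location for a scaled-down BP_Board, which then spawns its initial pieces.
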(event `InputTouch`
  (params (Location :type "Vector Structure") (FingerIndex :type "ETouchIndex Enum"))
  (bind (_locationx _locationy) (`PlayerController.GetInputTouchState` (`GameplayStatics.GetPlayerController` 0) "Touch1"))
  (bind _returnvalue (`KismetMathLibrary.MakeVector2D` _locationx _locationy))
  (:`Pressed`
    (bind (_outhit _returnvalue_2) (`self.WorldHitTest` _returnvalue))
    (if (not _returnvalue_2)
      (bind _returnvalue_3 (`ARBlueprintLibrary.LineTraceTrackedObjects` _returnvalue false false))
      (`/Engine/EditorBlueprintResources/StandardMacros.CompareInt` (`KismetArrayLibrary.Array_Length` _returnvalue_3)
        (:`>`
          (bind _returnvalue_4 (`|SpawnActorFromClass` "/Game/Blueprints/Board/BP_Board.BP_Board_C" (`KismetMathLibrary.MakeTransform` (.location (`ARTraceResultLibrary.GetLocalToWorldTransform` (`|GetArrayItem` _returnvalue_3))) (struct) (0.1 0.1 0.1)) "AlwaysSpawn" "OverrideRootScale" null null))
          (`/Game/Blueprints/Board/BP_Board.SpawnInitialPieces` _returnvalue_4 null null 0.0))))))

(fn `UserConstructionScript`)

(fn `WorldHitTest`
  (params (ScreenPosition :type "Vector2D Structure"))
  (returns (OutHit :type "HitResult Structure") (ReturnValue :type Boolean))
  (bind (_worldposition _worlddirection) (`GameplayStatics.DeprojectScreenToWorld` (`GameplayStatics.GetPlayerController` 0) ScreenPosition))
  (bind (_outhit _returnvalue) (`KismetSystemLibrary.LineTraceSingleForObjects` _worldposition (+ _worldposition (* _worlddirection 1000.0)) (`|MakeArray` "ObjectTypeQuery1" "ObjectTypeQuery2" "ObjectTypeQuery3" "ObjectTypeQuery4" "ObjectTypeQuery5" "ObjectTypeQuery6" :!type "EObjectTypeQuery Enum")))
  (return _outhit _returnvalue))