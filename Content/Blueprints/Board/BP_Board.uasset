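; Chess board actor that populates itself on BeginPlay with both sides' pieces and a grid of BP_Cell highlights, provided cell size and mesh height are set.
; Per-type functions feed a shared spawner, which picks color and mesh from each row's sign against the game mode's WhiteDirection.
; One helper converts signed grid coordinates, centered on the actor, into cell-center locations scaled by the board's X scale.
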(event `self.ReceiveBeginPlay`
  (if (and (> (`self.CellSideSize`) 0.0) (> (`self.MeshHeight`) 0.0))
    (`self.SpawnInitialPieces`)
    (`self.SpawnCellHighlights`)))

(fn `CalculatePieceLocation`
  (params (CoordinateX :type "Float (double-precision)") (CoordinateY :type "Float (double-precision)"))
  (returns (Location :type "Vector Structure"))
  (bind _x (.x (`self.GetActorScale3D`)))
  (bind _returnvalue (* _x (`self.CellSideSize`)))
  (bind _returnvalue_2 (/ _returnvalue 2.0))
  (return (+ (`KismetMathLibrary.MakeVector` (+ (* _returnvalue CoordinateX) _returnvalue_2) (+ _returnvalue_2 (* _returnvalue CoordinateY)) (* _x (`self.MeshHeight`))) (`self.K2_GetActorLocation`))))

(fn `SpawnBishops`
  (locals (CoordinatesX :type "Array of Float (double-precision)") (CoordinatesY :type "Array of Float (double-precision)"))
  (`self.SpawnSelectedPieces` "/Game/Blueprints/Pieces/BP_Bishop.BP_Bishop_C" "/Game/Assets/ChessSet/BishopBlack.BishopBlack" "/Game/Assets/ChessSet/BishopWhite.BishopWhite" (`local.CoordinatesX`) (`local.CoordinatesY`)))

(fn `SpawnCellHighlights`
  (for _index (range -4 4)
    (for _index_2 (range -4 4)
      (bind _location (`self.CalculatePieceLocation` (`KismetMathLibrary.Conv_IntToDouble` _index_2) (`KismetMathLibrary.Conv_IntToDouble` _index)))
      (`|SpawnActorFromClass` "/Game/Blueprints/Board/BP_Cell.BP_Cell_C" (`KismetMathLibrary.MakeTransform` (+ _location (0.0 0.0 1.0)) (struct) (`self.GetActorScale3D`)) "AlwaysSpawn" "OverrideRootScale" null null))))

(fn `SpawnInitialPieces`
  (`self.SpawnRooks`)
  (`self.SpawnKnights`)
  (`self.SpawnBishops`)
  (`self.SpawnQueens`)
  (`self.SpawnKings`)
  (`self.SpawnPawns`))

(fn `SpawnKings`
  (locals (CoordinatesX :type "Array of Float (double-precision)") (CoordinatesY :type "Array of Float (double-precision)"))
  (`self.SpawnSelectedPieces` "/Game/Blueprints/Pieces/BP_King.BP_King_C" "/Game/Assets/ChessSet/KingBlack.KingBlack" "/Game/Assets/ChessSet/KingWhite.KingWhite" (`local.CoordinatesX`) (`local.CoordinatesY`)))

(fn `SpawnKnights`
  (locals (CoordinatesX :type "Array of Float (double-precision)") (CoordinatesY :type "Array of Float (double-precision)"))
  (`self.SpawnSelectedPieces` "/Game/Blueprints/Pieces/BP_Knight.BP_Knight_C" "/Game/Assets/ChessSet/KnightBlack.KnightBlack" "/Game/Assets/ChessSet/KnightWhite.KnightWhite" (`local.CoordinatesX`) (`local.CoordinatesY`)))

(fn `SpawnPawns`
  (locals (CoordinatesX :type "Array of Float (double-precision)") (CoordinatesY :type "Array of Float (double-precision)"))
  (`self.SpawnSelectedPieces` "/Game/Blueprints/Pieces/BP_Pawn.BP_Pawn_C" "/Game/Assets/ChessSet/PawnBlack.PawnBlack" "/Game/Assets/ChessSet/PawnWhite.PawnWhite" (`local.CoordinatesX`) (`local.CoordinatesY`)))

(fn `SpawnQueens`
  (locals (CoordinatesX :type "Array of Float (double-precision)") (CoordinatesY :type "Array of Float (double-precision)"))
  (`self.SpawnSelectedPieces` "/Game/Blueprints/Pieces/BP_Queen.BP_Queen_C" "/Game/Assets/ChessSet/QueenBlack.QueenBlack" "/Game/Assets/ChessSet/QueenWhite.QueenWhite" (`local.CoordinatesX`) (`local.CoordinatesY`)))

(fn `SpawnRooks`
  (locals (CoordinatesX :type "Array of Float (double-precision)") (CoordinatesY :type "Array of Float (double-precision)"))
  (`self.SpawnSelectedPieces` "/Game/Blueprints/Pieces/BP_Rook.BP_Rook_C" "/Game/Assets/ChessSet/RookBlack.RookBlack" "/Game/Assets/ChessSet/RookWhite.RookWhite" (`local.CoordinatesX`) (`local.CoordinatesY`)))

(fn `SpawnSelectedPieces`
  (params (PieceClass :type "/Game/Blueprints/Pieces/BP_Piece Class Reference") (BlackMesh :type "StaticMesh Object Reference") (WhiteMesh :type "StaticMesh Object Reference") (CoordinatesX :type "Array of Float (double-precision)") (CoordinatesY :type "Array of Float (double-precision)"))
  (locals (Mesh :type "StaticMesh Object Reference") (IsCurrentWhite :type Boolean))
  (bind _asbp_chess_chantment_game_mode (cast `/Game/Blueprints/BP_ChessChantmentGameMode` (`GameplayStatics.GetGameMode`)))
  (for _array_element CoordinatesY
    (for _array_element_2 CoordinatesX
      (bind _location (`self.CalculatePieceLocation` _array_element_2 _array_element))
      (if (> (* _array_element (`/Game/Blueprints/BP_ChessChantmentGameMode.WhiteDirection` _asbp_chess_chantment_game_mode)) 0.0)
        (set `local.Mesh` (`local.BlackMesh`))
        (set `local.IsCurrentWhite` false)
        (else
          (set `local.Mesh` (`local.WhiteMesh`))
          (set `local.IsCurrentWhite` true)))
      (bind _returnvalue (`|SpawnActorFromClass` (`local.PieceClass`) (`KismetMathLibrary.MakeTransform` _location (struct) (`self.GetActorScale3D`)) "AlwaysSpawn" "OverrideRootScale" null null))
      (`StaticMeshComponent.SetStaticMesh` (`/Game/Blueprints/Pieces/BP_Piece.PieceMesh` _returnvalue) (`local.Mesh`))
      (set `/Game/Blueprints/Pieces/BP_Piece.IsWhite` (`local.IsCurrentWhite`) _returnvalue))))

(fn `UserConstructionScript`)