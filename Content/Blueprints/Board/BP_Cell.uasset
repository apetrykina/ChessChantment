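; BP_Cell is a clickable board cell for the ChessChantment chess game that serves as a move destination for the selected piece.
; Cursor and touch events swap hover and available materials, while a click or touch on a visible cell runs MoveSelectedPiece.
; It finds any occupant by overlap, deselecting the selected piece itself or removing an opposite-color piece.
; The GameMode's selected piece then teleports onto empty or captured cells and runs its post-move logic.
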(event `self.StaticMesh.OnBeginCursorOver`
  (params (TouchedComponent :type "PrimitiveComponent Object Reference"))
  (`PrimitiveComponent.SetMaterial` TouchedComponent 0 "/Game/Assets/M_Hover_Cell.M_Hover_Cell"))

(event `self.StaticMesh.OnEndCursorOver`
  (params (TouchedComponent :type "PrimitiveComponent Object Reference"))
  (`PrimitiveComponent.SetMaterial` TouchedComponent 0 "/Game/Assets/M_Available_Cell.M_Available_Cell"))

(event `self.StaticMesh.OnInputTouchBegin`
  (params (FingerIndex :type "ETouchIndex Enum" :default "Touch1") (TouchedComponent :type "PrimitiveComponent Object Reference"))
  (`PrimitiveComponent.SetMaterial` TouchedComponent 0 "/Game/Assets/M_Hover_Cell.M_Hover_Cell")
  (`self.MoveSelectedPiece` :!label _label))

(event `self.StaticMesh.OnClicked`
  (params (TouchedComponent :type "PrimitiveComponent Object Reference") (ButtonPressed :type "Key Structure"))
  (goto _label))

(event `self.StaticMesh.OnInputTouchEnd`
  (params (FingerIndex :type "ETouchIndex Enum" :default "Touch1") (TouchedComponent :type "PrimitiveComponent Object Reference"))
  (`PrimitiveComponent.SetMaterial` TouchedComponent 0 "/Game/Assets/M_Available_Cell.M_Available_Cell"))

(fn `MoveSelectedPiece`
  (bind _output (`|GetArrayItem` (`self.GetOverlappingActors` "/Game/Blueprints/Pieces/BP_Piece.BP_Piece_C")))
  (if (not (`self.bHidden`))
    (bind _asbp_chess_chantment_game_mode (cast `/Game/Blueprints/BP_ChessChantmentGameMode` (`GameplayStatics.GetGameMode`)))
    (bind _selectedpiece (`/Game/Blueprints/BP_ChessChantmentGameMode.SelectedPiece` _asbp_chess_chantment_game_mode))
    (if (`KismetSystemLibrary.IsValid` _selectedpiece)
      (if (== _selectedpiece _output)
        (`/Game/Blueprints/Pieces/BP_Piece.ClearPieceSelection` _selectedpiece)
        (else
          (bind _asbp_piece (cast `/Game/Blueprints/Pieces/BP_Piece` _output)
            (:`then`
              (if (xor (`/Game/Blueprints/Pieces/BP_Piece.IsWhite` _asbp_piece) (`/Game/Blueprints/Pieces/BP_Piece.IsWhite` _selectedpiece))
                (`self.K2_TeleportTo` :`self` _asbp_piece :`DestLocation` (+ (`self.K2_GetActorLocation`) (`KismetMathLibrary.MakeVector` 0.0 0.0 (* (`/Game/Blueprints/Board/BP_Board.CellSideSize` (`/Game/Blueprints/BP_ChessChantmentGameMode.Board` _asbp_chess_chantment_game_mode)) -1.0))))
                (`self.SetActorHiddenInGame` _asbp_piece true)
                (`self.K2_DestroyActor` _asbp_piece)
                (bind _returnvalue (`self.K2_TeleportTo` :`self` _selectedpiece :`DestLocation` (+ (`self.K2_GetActorLocation`) (0.0 0.0 -1.0)) :!label _label))
                (if _returnvalue
                  (`/Game/Blueprints/Pieces/BP_Piece.DoAfterMove` _selectedpiece)
                  (`/Game/Blueprints/Pieces/BP_Piece.ClearPieceSelection` _selectedpiece))))
            (:`CastFailed`
              (goto _label))))))))

(fn `UserConstructionScript`)