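; BP_Avatar is a character actor that players click or tap to choose as their avatar.
; When Clickable, selection sends its Id to BP_PlayerController through ServerSetPlayerAvatarId, then calls AfterAvatarChoice.
; Its skeletal mesh loops a staff idle animation from BeginPlay, with functions to swap its material and play a looping cast animation as a winner pose.
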(event `self.ReceiveBeginPlay`
  (`SkeletalMeshComponent.PlayAnimation` (`self.SkeletalMesh`) "/Game/Assets/Toony_Tiny_RTS_Set/Animations/Units/Staff/Anim_staff_01_idle.Anim_staff_01_idle" true))

(event `self.SkeletalMesh.OnClicked`
  (params (TouchedComponent :type "PrimitiveComponent Object Reference") (ButtonPressed :type "Key Structure"))
  (if (`self.Clickable`) :!label _label
    (bind _asbp_player_controller (cast `/Game/Blueprints/BP_PlayerController` (`GameplayStatics.GetPlayerController` 0)))
    (`/Game/Blueprints/BP_PlayerController.Server_SetPlayerAvatarId` _asbp_player_controller (`self.Id`))
    (`/Game/Blueprints/BP_PlayerController.AfterAvatarChoice` _asbp_player_controller)))

(event `self.SkeletalMesh.OnInputTouchBegin`
  (params (FingerIndex :type "ETouchIndex Enum" :default "Touch1") (TouchedComponent :type "PrimitiveComponent Object Reference"))
  (goto _label))

(fn `PlayWinnerAnimation`
  (`SkeletalMeshComponent.PlayAnimation` (`self.SkeletalMesh`) "/Game/Assets/Toony_Tiny_RTS_Set/Animations/Units/Staff/Anim_staff_07_cast_B.Anim_staff_07_cast_B" true))

(fn `SetMaterial`
  (params (NewMaterial :type "MaterialInstance Object Reference"))
  (if (`KismetSystemLibrary.IsValid` NewMaterial)
    (`PrimitiveComponent.SetMaterial` (`self.SkeletalMesh`) 0 NewMaterial)))

(fn `UserConstructionScript`)