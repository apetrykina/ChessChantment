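; Player controller for the networked ChessChantment chess game, linking the player's piece and match actions to the game mode.
; Enables mouse and touch input, then spawns a one-time overhead board camera after a short delay when SetCameraAbove is called.
; Server events check selection and ownership before moving pieces, and forward begin game, end move and end game to the game mode.
; Selection passes game-mode state to the client, which acts only for the active player.
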(event `self.ReceiveBeginPlay`
  (set `self.bEnableTouchEvents` true)
  (set `self.bEnableClickEvents` true)
  (set `self.bEnableMouseOverEvents` true))

(event `SetCameraAbove`
  (params (BoardTransform :type "Transform Structure"))
  (if (not (`self.CameraIsSet`))
    (`KismetSystemLibrary.Delay` 1.0)
    (bind _returnvalue (`|SpawnActorFromClass` "/Game/Blueprints/BP_CameraAbove.BP_CameraAbove_C" (`KismetMathLibrary.MakeTransform` (.location BoardTransform) (struct) (.scale BoardTransform)) "AlwaysSpawn" "OverrideRootScale" null null))
    (`self.SetViewTargetWithBlend` _returnvalue)
    (set `self.CameraIsSet` true)))

(event `Server_MovePiece`
  (params (Cell :type "/Game/Blueprints/Board/BP_Cell Object Reference") (Hidden :type Boolean))
  (if (not Hidden)
    (bind _asbp_chess_chantment_game_mode (cast `/Game/Blueprints/BP_ChessChantmentGameMode` (`GameplayStatics.GetGameMode`)))
    (bind _selectedpiece (`/Game/Blueprints/BP_ChessChantmentGameMode.SelectedPiece` _asbp_chess_chantment_game_mode))
    (if (and (`KismetSystemLibrary.IsValid` _selectedpiece) (== (`self.GetOwner` _selectedpiece) self))
      (`/Game/Blueprints/Board/BP_Cell.MoveSelectedPiece` Cell _selectedpiece))))

(event `Server_AuthorizeMove`
  (params (Piece :type "/Game/Blueprints/Pieces/BP_Piece Object Reference"))
  (bind _asbp_chess_chantment_game_mode (cast `/Game/Blueprints/BP_ChessChantmentGameMode` (`GameplayStatics.GetGameMode`)))
  (bind _pieceisinmove (`/Game/Blueprints/BP_ChessChantmentGameMode.PieceIsInMove` _asbp_chess_chantment_game_mode))
  (if (or _pieceisinmove (== self (`self.GetOwner` Piece)))
    (`self.Client_HandlePieceSelection` Piece (`/Game/Blueprints/BP_ChessChantmentGameMode.ActivePlayer` _asbp_chess_chantment_game_mode) (`/Game/Blueprints/BP_ChessChantmentGameMode.SelectedPiece` _asbp_chess_chantment_game_mode) _pieceisinmove (`/Game/Blueprints/BP_ChessChantmentGameMode.Board` _asbp_chess_chantment_game_mode) (`/Game/Blueprints/BP_ChessChantmentGameMode.WhiteDirection` _asbp_chess_chantment_game_mode))))

(event `Client_HandlePieceSelection`
  (params (ActivePiece :type "/Game/Blueprints/Pieces/BP_Piece Object Reference") (ActivePlayer :type "Actor Object Reference (by ref)") (SelectedPiece :type "/Game/Blueprints/Pieces/BP_Piece Object Reference (by ref)") (PieceInMove :type Boolean) (Board :type "/Game/Blueprints/Board/BP_Board Object Reference (by ref)") (WhiteDirection :type "Float (double-precision)"))
  (if (== ActivePlayer (`GameplayStatics.GetPlayerController` 0))
    (`/Game/Blueprints/Pieces/BP_Piece.HandlePieceSelection` ActivePiece SelectedPiece PieceInMove Board WhiteDirection)))

(event `Server_EndGame`
  (params (Instigator :type "Actor Object Reference"))
  (bind _asbp_chess_chantment_game_mode (cast `/Game/Blueprints/BP_ChessChantmentGameMode` (`GameplayStatics.GetGameMode`)))
  (`/Game/Blueprints/BP_ChessChantmentGameMode.EndGame` _asbp_chess_chantment_game_mode Instigator))

(event `Server_EndMove`
  (params (Instigator :type "Actor Object Reference"))
  (bind _asbp_chess_chantment_game_mode (cast `/Game/Blueprints/BP_ChessChantmentGameMode` (`GameplayStatics.GetGameMode`)))
  (`/Game/Blueprints/BP_ChessChantmentGameMode.EndMove` _asbp_chess_chantment_game_mode Instigator))

(event `Server_BeginGame`
  (params (Instigator :type "Controller Object Reference"))
  (bind _asbp_chess_chantment_game_mode (cast `/Game/Blueprints/BP_ChessChantmentGameMode` (`GameplayStatics.GetGameMode`)))
  (`/Game/Blueprints/BP_ChessChantmentGameMode.BeginGame` _asbp_chess_chantment_game_mode Instigator))

(fn `UserConstructionScript`)