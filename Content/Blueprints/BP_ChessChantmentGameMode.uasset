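; Game mode for a two-player chess game that manages players, turns and game end.
; BeginGame ensures a board exists outside AR, sets an overhead camera, then registers players and spawns pieces once the second joins, with White first.
; EndMove passes the turn from the active player, while EndGame destroys all pieces and announces the winner.
; AR session start and geometry debug drawing exist but are disconnected, though AR mode branches remain.
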(event `self.ReceiveTick`
  (params (DeltaSeconds :type "Float (single-precision)")))

(event `self.ReceiveBeginPlay`)

(fn `BeginGame`
  (params (Player :type "Actor Object Reference"))
  (bind _players (`self.Players`))
  (bind _returnvalue (`KismetArrayLibrary.Array_Length` (`self.Players`)))
  (if (not (`KismetSystemLibrary.IsValid` (`self.Board`)))
    (`self.SpawnBoard`))
  (if (not (`self.ARModeActive`))
    (bind _asbp_player_controller (cast `/Game/Blueprints/BP_PlayerController` (`local.Player`)))
    (`/Game/Blueprints/BP_PlayerController.SetCameraAbove` _asbp_player_controller (`self.GetTransform` (`self.Board`))))
  (if (== _returnvalue 0)
    (`KismetArrayLibrary.Array_Add` _players _asbp_player_controller)
    (elif (and (> _returnvalue 0) (< _returnvalue 2))
      (`KismetArrayLibrary.Array_Add` _players _asbp_player_controller)
      (bind _output_get (set `self.WhitePlayer` (`|GetArrayItem` _players)))
      (bind _output_get_2 (set `self.BlackPlayer` (`|GetArrayItem` _players 1)))
      (`/Game/Blueprints/Board/BP_Board.SpawnInitialPieces` (`self.Board`) _output_get_2 _output_get (`self.WhiteDirection`))
      (set `self.ActivePlayer` (`self.WhitePlayer`))
      (`KismetSystemLibrary.PrintString` "White turn!" true true (struct :`G` 0.66 :`B` 1.0 :`A` 1.0) 3.0))))

(fn `ClearAllPieces`
  (bind _outactors (`GameplayStatics.GetAllActorsOfClass` "/Game/Blueprints/Pieces/BP_Piece.BP_Piece_C"))
  (for _array_element _outactors
    (`self.K2_DestroyActor` _array_element)))

(fn `EndGame`
  (params (Instigator :type "Actor Object Reference"))
  (`self.ClearAllPieces`)
  (if (== (`self.WhitePlayer`) Instigator)
    (`KismetSystemLibrary.PrintString` "White win!" true true (struct :`R` 0.803922 :`G` 0.2 :`B` 1.0 :`A` 1.0) 60.0)
    (else
      (`KismetSystemLibrary.PrintString` "Black win!" true true (struct :`R` 0.803922 :`G` 0.2 :`B` 1.0 :`A` 1.0) 60.0))))

(fn `EndMove`
  (params (Instigator :type "Actor Object Reference"))
  (bind _whiteplayer (`self.WhitePlayer`))
  (if (== (`self.ActivePlayer`) Instigator)
    (if (== _whiteplayer Instigator)
      (set `self.ActivePlayer` (`self.BlackPlayer`))
      (`KismetSystemLibrary.PrintString` "Black turn!" true true (struct :`G` 0.66 :`B` 1.0 :`A` 1.0) 3.0)
      (else
        (set `self.ActivePlayer` _whiteplayer)
        (`KismetSystemLibrary.PrintString` "White turn!" true true (struct :`G` 0.66 :`B` 1.0 :`A` 1.0) 3.0)))))

(fn `SpawnBoard`
  (locals (BoardTransform :type "Transform Structure"))
  (if (not (`self.ARModeActive`))
    (set `local.BoardTransform` (`KismetMathLibrary.MakeTransform` (0.0 0.0 0.0)))
    (bind _returnvalue (`|SpawnActorFromClass` "/Game/Blueprints/Board/BP_Board.BP_Board_C" (`local.BoardTransform`) "Undefined" "OverrideRootScale" null null))
    (set `self.Board` _returnvalue)))

(fn `UserConstructionScript`)