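; Base chess piece Actor that handles hover and touch cell highlighting, selection and its color-based mesh.
; Clicks or touches request authorization through BP_PlayerController; selection stores state in BP_ChessChantmentGameMode and unhides available cells.
; Available cells come from direction-aware multi line traces over cell offsets, stopping at the first piece and dropping its cell if friendly.
; Selecting a piece while another is in move requests a move onto its cell.
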(event `self.PieceMesh.OnBeginCursorOver`
  (params (TouchedComponent :type "PrimitiveComponent Object Reference"))
  (bind _overlappingactors (`self.GetOverlappingActors` "/Game/Blueprints/Board/BP_Cell.BP_Cell_C"))
  (if (> (`KismetArrayLibrary.Array_Length` _overlappingactors) 0) :!label _label
    (`PrimitiveComponent.SetMaterial` (`self.GetComponentByClass` (`|GetArrayItem` _overlappingactors) "/Script/Engine.StaticMeshComponent") 0 "/Game/Assets/M_Hover_Cell.M_Hover_Cell")))

(event `self.PieceMesh.OnInputTouchBegin`
  (params (FingerIndex :type "ETouchIndex Enum" :default "Touch1") (TouchedComponent :type "PrimitiveComponent Object Reference"))
  (`self.OnPieceSelected`)
  (goto _label))

(event `self.PieceMesh.OnInputTouchEnd`
  (params (FingerIndex :type "ETouchIndex Enum" :default "Touch1") (TouchedComponent :type "PrimitiveComponent Object Reference"))
  (bind _overlappingactors (`self.GetOverlappingActors` "/Game/Blueprints/Board/BP_Cell.BP_Cell_C"))
  (if (> (`KismetArrayLibrary.Array_Length` _overlappingactors) 0) :!label _label_2
    (`PrimitiveComponent.SetMaterial` (`self.GetComponentByClass` (`|GetArrayItem` _overlappingactors) "/Script/Engine.StaticMeshComponent") 0 "/Game/Assets/M_Available_Cell.M_Available_Cell")))

(event `self.PieceMesh.OnEndCursorOver`
  (params (TouchedComponent :type "PrimitiveComponent Object Reference"))
  (goto _label_2))

(event `self.PieceMesh.OnClicked`
  (params (TouchedComponent :type "PrimitiveComponent Object Reference") (ButtonPressed :type "Key Structure"))
  (`self.OnPieceSelected`))

(event `SetCorrectMesh`
  (`self.SetMesh`))

(event `ChangeLocation`
  (params (NewLocation :type "Vector Structure"))
  (`self.K2_SetActorLocation` NewLocation))

(event `Server_SetSelectedPiece`
  (params (NewSelected :type "/Game/Blueprints/Pieces/BP_Piece Object Reference"))
  (bind _asbp_chess_chantment_game_mode (cast `/Game/Blueprints/BP_ChessChantmentGameMode` (`GameplayStatics.GetGameMode`)))
  (set `/Game/Blueprints/BP_ChessChantmentGameMode.SelectedPiece` NewSelected _asbp_chess_chantment_game_mode))

(event `Server_SetPieceInMove`
  (params (InMove :type Boolean))
  (bind _asbp_chess_chantment_game_mode (cast `/Game/Blueprints/BP_ChessChantmentGameMode` (`GameplayStatics.GetGameMode`)))
  (set `/Game/Blueprints/BP_ChessChantmentGameMode.PieceIsInMove` InMove _asbp_chess_chantment_game_mode))

(event `Server_SetAvailableCells`
  (params (AvailableCells :type "Array of /Game/Blueprints/Board/BP_Cell Object Reference"))
  (set `self.AvailableCells` AvailableCells))

(event `Server_SetCellVisibility`
  (params (Cell :type "/Game/Blueprints/Board/BP_Cell Object Reference") (Hidden :type Boolean))
  (`self.SetActorHiddenInGame` Cell Hidden))

(fn `ClearPieceSelection`
  (params (TargetClient :type "Actor Object Reference (by ref)"))
  (bind _availablecells (`self.AvailableCells`))
  (for _array_element _availablecells
    (cast `/Game/Blueprints/BP_PlayerController` (`GameplayStatics.GetPlayerController` 0))
    (`self.Server_SetCellVisibility` _array_element true))
  (`KismetArrayLibrary.Array_Clear` _availablecells)
  (`self.Server_SetPieceInMove` false)
  (`self.Server_SetSelectedPiece` null))

(fn `DoAfterMove`
  (if (not (`self.HasMoved`))
    (set `self.HasMoved` true)))

(fn `GetAvailableCellsWithOffsets`
  (params (EndCellOffsets :type "Array of Vector2D Structure (by ref)") (Board :type "/Game/Blueprints/Board/BP_Board Object Reference (by ref)") (WhiteDirection :type "Float (double-precision)"))
  (returns (AvailableCells :type "Array of /Game/Blueprints/Board/BP_Cell Object Reference"))
  (locals (PieceAvailableCells :type "Array of /Game/Blueprints/Board/BP_Cell Object Reference") (HitEnemyPiece :type Boolean))
  (bind _pieceavailablecells (`local.PieceAvailableCells`))
  (bind _piecedirection (`self.GetPieceDirection` WhiteDirection))
  (for _array_element (`local.EndCellOffsets`)
    (bind _lineend (`self.GetLineTraceEndLocation` (`/Game/Blueprints/Board/BP_Board.CellSideSize` Board) _piecedirection _array_element))
    (bind _outhits (`KismetSystemLibrary.LineTraceMultiForObjects` (+ (`self.K2_GetActorLocation`) (0.0 0.0 1.0)) _lineend (`|MakeArray` "ObjectTypeQuery2" :!type "EObjectTypeQuery Enum") false (`|MakeArray` Board :!type "Actor Object Reference")))
    (for _array_element_2 _outhits
      (bind (_bblockinghit _binitialoverlap _time _distance _location _impactpoint _normal _impactnormal _physmat _hitactor) (`GameplayStatics.BreakHitResult` _array_element_2))
      (bind _asbp_cell (cast `/Game/Blueprints/Board/BP_Cell` _hitactor)
        (:`then`
          (`KismetArrayLibrary.Array_Add` (`local.PieceAvailableCells`) _asbp_cell))
        (:`CastFailed`
          (bind _asbp_piece (cast `/Game/Blueprints/Pieces/BP_Piece` _hitactor))
          (if (xor (`/Game/Blueprints/Pieces/BP_Piece.IsWhite` _asbp_piece) (`self.IsWhite`))
            (break)
            (else
              (`KismetArrayLibrary.Array_Remove` _pieceavailablecells (`KismetArrayLibrary.Array_LastIndex` _pieceavailablecells))
              (break)))))))
  (return (`local.PieceAvailableCells`)))

(fn `GetLineTraceEndLocation`
  (params (BoardCellSize :type "Float (double-precision)") (Direction :type "Float (double-precision)") (EndCellOffset :type "Vector2D Structure"))
  (returns (LineEnd :type "Vector Structure"))
  (bind (_x _y) (`KismetMathLibrary.BreakVector2D` EndCellOffset))
  (return (`KismetMathLibrary.MakeVector` (+ (* BoardCellSize (* Direction _x)) (.x (`self.K2_GetActorLocation`))) (+ (.y (`self.K2_GetActorLocation`)) (* BoardCellSize (* Direction _y))) (+ (.z (`self.K2_GetActorLocation`)) 1.0))))

(fn `GetPieceAvailableCells`
  (params (Board :type "/Game/Blueprints/Board/BP_Board Object Reference (by ref)") (WhiteDirection :type "Float (double-precision)"))
  (returns (AvailableCells :type "Array of /Game/Blueprints/Board/BP_Cell Object Reference"))
  (bind _availablecells (`self.GetAvailableCellsWithOffsets` (`|MakeArray` (0.5 0.5) :!type "Vector2D Structure") Board WhiteDirection))
  (return _availablecells))

(fn `GetPieceDirection`
  (params (GameWhiteDirection :type "Float (double-precision)" :default 1.0))
  (returns (PieceDirection :type "Float (double-precision)"))
  (if (`self.IsWhite`)
    (return GameWhiteDirection)
    (else
      (return (* GameWhiteDirection -1.0)))))

(fn `HandlePieceSelection`
  (params (SelectedPiece :type "/Game/Blueprints/Pieces/BP_Piece Object Reference") (PieceInMove :type Boolean) (Board :type "/Game/Blueprints/Board/BP_Board Object Reference") (WhiteDirection :type "Float (double-precision)"))
  (if (`KismetSystemLibrary.IsValid` SelectedPiece)
    (if (and (!= SelectedPiece self) PieceInMove)
      (bind _asbp_cell (cast `/Game/Blueprints/Board/BP_Cell` (`|GetArrayItem` (`self.GetOverlappingActors` "/Game/Blueprints/Board/BP_Cell.BP_Cell_C"))))
      (bind _asbp_player_controller (cast `/Game/Blueprints/BP_PlayerController` (`GameplayStatics.GetPlayerController` 0)))
      (`/Game/Blueprints/BP_PlayerController.Server_MovePiece` _asbp_player_controller _asbp_cell (`Actor.bHidden` _asbp_cell))
      (else
        (`self.SelectPiece` (`local.SelectedPiece`) (`local.Board`) (`local.WhiteDirection`) :!label _label)))
    (else
      (goto _label))))

(fn `OnPieceSelected`
  (bind _overlappingactors (`self.GetOverlappingActors` "/Game/Blueprints/Board/BP_Cell.BP_Cell_C"))
  (bind _asbp_player_controller (cast `/Game/Blueprints/BP_PlayerController` (`GameplayStatics.GetPlayerController` 0)))
  (`/Game/Blueprints/BP_PlayerController.Server_AuthorizeMove` _asbp_player_controller self)
  (if (> (`KismetArrayLibrary.Array_Length` _overlappingactors) 0)
    (`PrimitiveComponent.SetMaterial` (`self.GetComponentByClass` (`|GetArrayItem` _overlappingactors) "/Script/Engine.StaticMeshComponent") 0 "/Game/Assets/M_Hover_Cell.M_Hover_Cell")))

(fn `SelectPiece`
  (params (SelectedPiece :type "/Game/Blueprints/Pieces/BP_Piece Object Reference") (Board :type "/Game/Blueprints/Board/BP_Board Object Reference (by ref)") (WhiteDirection :type "Float (double-precision)"))
  (bind _returnvalue (`GameplayStatics.GetPlayerController` 0))
  (if (== SelectedPiece self)
    (`self.ClearPieceSelection` _returnvalue)
    (else
      (if (`KismetSystemLibrary.IsValid` SelectedPiece)
        (`self.ClearPieceSelection` SelectedPiece _returnvalue))
      (`self.Server_SetSelectedPiece` self)
      (bind _availablecells (`self.GetPieceAvailableCells` (`local.Board`) (`local.WhiteDirection`)))
      (`self.Server_SetAvailableCells` _availablecells)
      (for _array_element _availablecells
        (`self.Server_SetCellVisibility` _array_element))
      (`self.Server_SetPieceInMove` true))))

(fn `SetMesh`
  (bind _piecemesh (`self.PieceMesh`))
  (if (`self.IsWhite`)
    (`StaticMeshComponent.SetStaticMesh` _piecemesh (`self.WhiteMesh`))
    (else
      (`StaticMeshComponent.SetStaticMesh` _piecemesh (`self.BlackMesh`)))))

(fn `UserConstructionScript`)