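; Knight chess piece that computes the cells it can move to on the board.
; GetPieceAvailableCells line-traces toward each of the eight L-shaped offsets, scaled by board cell size and oriented by piece direction from the game mode.
; It keeps only the hit cell at each trace endpoint, then removes cells holding same-colour pieces while iterating the array.
; The knight's current cell is appended to the returned list.
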(fn `GetPieceAvailableCells`
  (returns (AvailableCells :type "Array of /Game/Blueprints/Board/BP_Cell Object Reference"))
  (locals (PieceAvailableCells :type "Array of /Game/Blueprints/Board/BP_Cell Object Reference") (PathCells :type "Array of /Game/Blueprints/Board/BP_Cell Object Reference"))
  (bind _overlappingactors (`self.GetOverlappingActors` "/Game/Blueprints/Board/BP_Cell.BP_Cell_C"))
  (bind _pathcells (`local.PathCells`))
  (bind _asbp_chess_chantment_game_mode (cast `/Game/Blueprints/BP_ChessChantmentGameMode` (`GameplayStatics.GetGameMode`)))
  (bind _piecedirection (`self.GetPieceDirection` (`/Game/Blueprints/BP_ChessChantmentGameMode.WhiteDirection` _asbp_chess_chantment_game_mode)))
  (for _array_element (`|MakeArray` (-2.0 -1.0) (-2.0 1.0) (-1.0 -2.0) (-1.0 2.0) (1.0 -2.0) (1.0 2.0) (2.0 -1.0) (2.0 1.0) :!type "Vector2D Structure")
    (bind _lineend (`self.GetLineTraceEndLocation` (`/Game/Blueprints/Board/BP_Board.CellSideSize` (`/Game/Blueprints/BP_ChessChantmentGameMode.Board` _asbp_chess_chantment_game_mode)) _piecedirection _array_element))
    (bind _outhits (`KismetSystemLibrary.LineTraceMultiForObjects` (+ (`self.K2_GetActorLocation`) (0.0 0.0 1.0)) _lineend (`|MakeArray` "ObjectTypeQuery2" :!type "EObjectTypeQuery Enum")))
    (for _array_element_2 _outhits
      (bind _asbp_cell (cast `/Game/Blueprints/Board/BP_Cell` (`.HitActor` (`GameplayStatics.BreakHitResult` _array_element_2))))
      (`KismetArrayLibrary.Array_Add` (`local.PathCells`) _asbp_cell))
    (`KismetArrayLibrary.Array_Reverse` _pathcells)
    (for _array_element_3 _pathcells
      (if (== (`self.K2_GetActorLocation` _array_element_3) _lineend)
        (`KismetArrayLibrary.Array_Add` (`local.PieceAvailableCells`) _array_element_3)
        (break)))
    (`KismetArrayLibrary.Array_Clear` (`local.PathCells`)))
  (for (_array_element_4 _array_index) (`local.PieceAvailableCells`)
    (bind _overlappingactors_2 (`self.GetOverlappingActors` _array_element_4 "/Game/Blueprints/Pieces/BP_Piece.BP_Piece_C"))
    (if (> (`KismetArrayLibrary.Array_Length` _overlappingactors_2) 0)
      (bind _asbp_piece (cast `/Game/Blueprints/Pieces/BP_Piece` (`|GetArrayItem` _overlappingactors_2)))
      (if (not (xor (`/Game/Blueprints/Pieces/BP_Piece.IsWhite` _asbp_piece) (`self.IsWhite`)))
        (`KismetArrayLibrary.Array_Remove` (`local.PieceAvailableCells`) _array_index))))
  (if (> (`KismetArrayLibrary.Array_Length` _overlappingactors) 0)
    (bind _asbp_cell_2 (cast `/Game/Blueprints/Board/BP_Cell` (`|GetArrayItem` _overlappingactors))
      (:`then`
        (`KismetArrayLibrary.Array_Add` (`local.PieceAvailableCells`) _asbp_cell_2))
      (:`CastFailed`
        _)))
  (return (`local.PieceAvailableCells`)))

(fn `UserConstructionScript`
  (`parent.UserConstructionScript`))