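; BP_Pawn is the pawn piece in ChessChantment, defining which board cells it can move to.
; GetPieceAvailableCells builds end offsets: two cells forward before the first move, one afterwards, plus each forward diagonal where a line trace hits a BP_Piece.
; Inherited helpers handle direction and turn these offsets into available cells.
; DoAfterMove extends the parent to set HasMoved, ending the double step.
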(fn `DoAfterMove`
  (`parent.DoAfterMove`)
  (if (not (`self.HasMoved`))
    (set `self.HasMoved` true)))

(fn `GetPieceAvailableCells`
  (returns (AvailableCells :type "Array of /Game/Blueprints/Board/BP_Cell Object Reference"))
  (locals (EndCellOffsets :type "Array of Vector2D Structure") (CurrentOffset :type "Vector2D Structure"))
  (bind _endcelloffsets (`local.EndCellOffsets`))
  (if (`self.HasMoved`)
    (`KismetArrayLibrary.Array_Add` _endcelloffsets (0.0 1.0))
    (else
      (`KismetArrayLibrary.Array_Add` _endcelloffsets (0.0 2.0))))
  (bind _asbp_chess_chantment_game_mode (cast `/Game/Blueprints/BP_ChessChantmentGameMode` (`GameplayStatics.GetGameMode`)))
  (for _array_element (`|MakeArray` -1.0 1.0 :!type "Float (single-precision)")
    (bind _returnvalue (`KismetMathLibrary.MakeVector2D` _array_element 1.0))
    (set `local.CurrentOffset` _returnvalue)
    (bind _piecedirection (`self.GetPieceDirection` 1.0))
    (bind _lineend (`self.GetLineTraceEndLocation` (`/Game/Blueprints/Board/BP_Board.CellSideSize` (`/Game/Blueprints/BP_ChessChantmentGameMode.Board` _asbp_chess_chantment_game_mode)) _piecedirection _returnvalue))
    (bind _outhits (`KismetSystemLibrary.LineTraceMultiForObjects` (`self.K2_GetActorLocation`) _lineend (`|MakeArray` "ObjectTypeQuery2" :!type "EObjectTypeQuery Enum")))
    (for _array_element_2 _outhits
      (cast `/Game/Blueprints/Pieces/BP_Piece` (`.HitActor` (`GameplayStatics.BreakHitResult` _array_element_2)))
      (`KismetArrayLibrary.Array_Add` (`local.EndCellOffsets`) (`local.CurrentOffset`))
      (break)))
  (bind _availablecells (`self.GetAvailableCellsWithOffsets` (`local.EndCellOffsets`)))
  (return _availablecells))

(fn `UserConstructionScript`
  (`parent.UserConstructionScript`))